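; AtmosphereBP sets up a planet atmosphere with Rayleigh, Mie or combined scattering in its construction script.
; It picks sky and surface materials by quality, scattering type and lighting, unless overridden, then pushes radius, light, scattering and texture parameters to dynamic instances.
; Scattering values scale with planet radius, keeping the look size-independent.
; The outer radius, where exponential density falls to CutoffDensity, also drives mesh scale.
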(fn `CalcOuterRadius`
  (params (InnerRadius :type "Float (double-precision)" :default 0.0))
  (returns (OuterRadius :type "Float (double-precision)"))
  (bind _outerradius (`self.CalcOuterRadiusForLayer` InnerRadius (`self.MieScattering`)))
  (bind _outerradius_2 (`self.CalcOuterRadiusForLayer` InnerRadius (`self.RayleighScattering`)))
  (return (select `/Game/AtmosphereV2/System/Blueprints/AtmoBP_ScatteringType` (`self.ScatteringType`) :`NewEnumerator0` _outerradius_2 :`NewEnumerator1` _outerradius :`NewEnumerator2` (select `bool` (`self.UseMieLayerDensity`) :`false` _outerradius_2 :`true` _outerradius))))

(fn `CalcOuterRadiusForLayer`
  (params (InnerRadius :type "Float (double-precision)" :default 0.0) (ScatteringParameters :type "/Game/AtmosphereV2/System/Blueprints/AtmoBP_Scattering Structure"))
  (returns (OuterRadius :type "Float (double-precision)"))
  (return (- InnerRadius (* (`.FinalScaleHeight` (`self.CalcScatteringParameters` ScatteringParameters)) (`KismetMathLibrary.Loge` (`self.CutoffDensity`))))))

(fn `CalcScatteringParameters`
  (params (Parameters :type "/Game/AtmosphereV2/System/Blueprints/AtmoBP_Scattering Structure"))
  (returns (FinalScatter :type "Object.LinearColor Structure") (FinalAttenuation :type "Object.LinearColor Structure") (FinalScaleHeight :type "Float (double-precision)"))
  (bind _returnvalue (/ (`self.UnitRadius`) (`self.GetActualPlanetRadius`)))
  (bind _returnvalue_2 (* Parameters_Density_18_D71424EE464B7BD773AA38B5D312E66E (`self.MasterDensity`)))
  (return (* (* (* Parameters_Scatter_3_0828DEB54586715A7672C7AEFEF338BE Parameters_ScatterDensity_9_837100DD483E58C433783CA780D2C960) _returnvalue_2) _returnvalue) (* (* (* Parameters_Attenuation_6_99FD3B9947101F196939CFBA935DB0A2 Parameters_AttenuationDensity_12_BDD6C3824E224A65BFD027A07525E379) _returnvalue_2) _returnvalue) (/ Parameters_ScaleHeight_15_8821A0E545F2D368F037008FEB94E2B1 _returnvalue)))

(fn `GetActualPlanetRadius`
  (returns (Radius :type "Float (double-precision)"))
  (return (* (`self.MakeUniformSize` (`self.GetActorScale3D`)) (select `bool` (`self.OverridePlanetRadius`) :`false` (`self.MakeUniformSize` (`.Max` (`StaticMeshComponent.GetLocalBounds`))) :`true` (`self.PlanetRadiusOverrideValue`)))))

(fn `InitMaterialParameters`
  (params (MaterialInstance :type "MaterialInstanceDynamic Object Reference") (InnerRadius :type "Float (double-precision)" :default 0.0) (OuterRadius :type "Float (double-precision)" :default 0.0))
  (`|ExecutionSequence`
    (:`then_0`
      (`self.SetMaterialRadius` MaterialInstance InnerRadius OuterRadius))
    (:`then_1`
      (`self.SetMaterialLight` MaterialInstance))
    (:`then_2`
      (`self.SetMaterialScattering` MaterialInstance))
    (:`then_3`
      (`MaterialInstanceDynamic.SetTextureParameterValue` MaterialInstance "SurfaceTexture" (`self.SurfaceTexture`)))))

(fn `InitMaterials`
  (returns (SkyMI :type "MaterialInstanceDynamic Object Reference") (SurfaceMI :type "MaterialInstanceDynamic Object Reference"))
  (bind _skymaterialoverride (`self.SkyMaterialOverride`))
  (bind _surfacematerialoverride (`self.SurfaceMaterialOverride`))
  (`|ExecutionSequence`
    (:`then_0`
      (bind _returnvalue (`PrimitiveComponent.CreateDynamicMaterialInstance` 0 (select `bool` (`KismetSystemLibrary.IsValid` _skymaterialoverride) :`false` (select `/Game/AtmosphereV2/System/Blueprints/AtmoBP_Quality` (`self.Quality`) :`NewEnumerator0` (`self.SelectSkyMaterial_High`) :`NewEnumerator1` (`self.SelectSkyMaterial_Medium`) :`NewEnumerator2` (`self.SelectSkyMaterial_Low`)) :`true` _skymaterialoverride))))
    (:`then_1`
      (bind _returnvalue_2 (`PrimitiveComponent.CreateDynamicMaterialInstance` 0 (select `bool` (`KismetSystemLibrary.IsValid` _surfacematerialoverride) :`false` (select `/Game/AtmosphereV2/System/Blueprints/AtmoBP_Quality` (`self.Quality`) :`NewEnumerator0` (`self.SelectSurfMaterial_High`) :`NewEnumerator1` (`self.SelectSurfMaterial_Medium`) :`NewEnumerator2` (`self.SelectSurfMaterial_Low`)) :`true` _surfacematerialoverride))))
    (:`then_2`
      (return _returnvalue _returnvalue_2))))

(fn `MakeUniformSize`
  (params (NonUniformSize :type "Object.Vector Structure" :default (0.0 0.0 0.0)))
  (returns (UniformSize :type "Float (double-precision)"))
  (return (/ (+ (.x NonUniformSize) (.y NonUniformSize) (.z NonUniformSize)) 3.0)))

(fn `SelectSkyMaterial_High`
  (returns (Material :type "MaterialInterface Object Reference"))
  (bind _scatteringtype (`self.ScatteringType`))
  (return (select `bool` (`self.EnableLighting`) :`false` (select `/Game/AtmosphereV2/System/Blueprints/AtmoBP_ScatteringType` _scatteringtype :`NewEnumerator0` "/Game/AtmosphereV2/MaterialInstances/High/Sky_R_Hi.Sky_R_Hi" :`NewEnumerator1` "/Game/AtmosphereV2/MaterialInstances/High/Sky_M_Hi.Sky_M_Hi" :`NewEnumerator2` "/Game/AtmosphereV2/MaterialInstances/High/Sky_RM_Hi.Sky_RM_Hi" :!type "MaterialInterface Object Reference") :`true` (select `/Game/AtmosphereV2/System/Blueprints/AtmoBP_ScatteringType` _scatteringtype :`NewEnumerator0` "/Game/AtmosphereV2/MaterialInstances/High/Sky_RL_Hi.Sky_RL_Hi" :`NewEnumerator1` "/Game/AtmosphereV2/MaterialInstances/High/Sky_ML_Hi.Sky_ML_Hi" :`NewEnumerator2` "/Game/AtmosphereV2/MaterialInstances/High/Sky_RML_Hi.Sky_RML_Hi" :!type "MaterialInterface Object Reference"))))

(fn `SelectSkyMaterial_Low`
  (returns (Material :type "MaterialInterface Object Reference"))
  (bind _scatteringtype (`self.ScatteringType`))
  (return (select `bool` (`self.EnableLighting`) :`false` (select `/Game/AtmosphereV2/System/Blueprints/AtmoBP_ScatteringType` _scatteringtype :`NewEnumerator0` "/Game/AtmosphereV2/MaterialInstances/Low/Sky_R_Lo.Sky_R_Lo" :`NewEnumerator1` "/Game/AtmosphereV2/MaterialInstances/Low/Sky_M_Lo.Sky_M_Lo" :`NewEnumerator2` "/Game/AtmosphereV2/MaterialInstances/Low/Sky_RM_Lo.Sky_RM_Lo" :!type "MaterialInterface Object Reference") :`true` (select `/Game/AtmosphereV2/System/Blueprints/AtmoBP_ScatteringType` _scatteringtype :`NewEnumerator0` "/Game/AtmosphereV2/MaterialInstances/Low/Sky_RL_Lo.Sky_RL_Lo" :`NewEnumerator1` "/Game/AtmosphereV2/MaterialInstances/Low/Sky_ML_Lo.Sky_ML_Lo" :`NewEnumerator2` "/Game/AtmosphereV2/MaterialInstances/Low/Sky_RML_Lo.Sky_RML_Lo" :!type "MaterialInterface Object Reference"))))

(fn `SelectSkyMaterial_Medium`
  (returns (Material :type "MaterialInterface Object Reference"))
  (bind _scatteringtype (`self.ScatteringType`))
  (return (select `bool` (`self.EnableLighting`) :`false` (select `/Game/AtmosphereV2/System/Blueprints/AtmoBP_ScatteringType` _scatteringtype :`NewEnumerator0` "/Game/AtmosphereV2/MaterialInstances/Medium/Sky_R_Mid.Sky_R_Mid" :`NewEnumerator1` "/Game/AtmosphereV2/MaterialInstances/Medium/Sky_M_Mid.Sky_M_Mid" :`NewEnumerator2` "/Game/AtmosphereV2/MaterialInstances/Medium/Sky_RM_Mid.Sky_RM_Mid" :!type "MaterialInterface Object Reference") :`true` (select `/Game/AtmosphereV2/System/Blueprints/AtmoBP_ScatteringType` _scatteringtype :`NewEnumerator0` "/Game/AtmosphereV2/MaterialInstances/Medium/Sky_RL_Mid.Sky_RL_Mid" :`NewEnumerator1` "/Game/AtmosphereV2/MaterialInstances/Medium/Sky_ML_Mid.Sky_ML_Mid" :`NewEnumerator2` "/Game/AtmosphereV2/MaterialInstances/Medium/Sky_RML_Mid.Sky_RML_Mid" :!type "MaterialInterface Object Reference"))))

(fn `SelectSurfMaterial_High`
  (returns (Material :type "MaterialInterface Object Reference"))
  (bind _scatteringtype (`self.ScatteringType`))
  (return (select `bool` (`self.EnableLighting`) :`false` (select `/Game/AtmosphereV2/System/Blueprints/AtmoBP_ScatteringType` _scatteringtype :`NewEnumerator0` "/Game/AtmosphereV2/MaterialInstances/High/Surf_R_Hi.Surf_R_Hi" :`NewEnumerator1` "/Game/AtmosphereV2/MaterialInstances/High/Surf_M_Hi.Surf_M_Hi" :`NewEnumerator2` "/Game/AtmosphereV2/MaterialInstances/High/Surf_RM_Hi.Surf_RM_Hi" :!type "MaterialInterface Object Reference") :`true` (select `/Game/AtmosphereV2/System/Blueprints/AtmoBP_ScatteringType` _scatteringtype :`NewEnumerator0` "/Game/AtmosphereV2/MaterialInstances/High/Surf_RL_Hi.Surf_RL_Hi" :`NewEnumerator1` "/Game/AtmosphereV2/MaterialInstances/High/Surf_ML_Hi.Surf_ML_Hi" :`NewEnumerator2` "/Game/AtmosphereV2/MaterialInstances/High/Surf_RML_Hi.Surf_RML_Hi" :!type "MaterialInterface Object Reference"))))

(fn `SelectSurfMaterial_Low`
  (returns (Material :type "MaterialInterface Object Reference"))
  (bind _scatteringtype (`self.ScatteringType`))
  (return (select `bool` (`self.EnableLighting`) :`false` (select `/Game/AtmosphereV2/System/Blueprints/AtmoBP_ScatteringType` _scatteringtype :`NewEnumerator0` "/Game/AtmosphereV2/MaterialInstances/Low/Surf_R_Lo.Surf_R_Lo" :`NewEnumerator1` "/Game/AtmosphereV2/MaterialInstances/Low/Surf_M_Lo.Surf_M_Lo" :`NewEnumerator2` "/Game/AtmosphereV2/MaterialInstances/Low/Surf_RM_Lo.Surf_RM_Lo" :!type "MaterialInterface Object Reference") :`true` (select `/Game/AtmosphereV2/System/Blueprints/AtmoBP_ScatteringType` _scatteringtype :`NewEnumerator0` "/Game/AtmosphereV2/MaterialInstances/Low/Surf_RL_Lo.Surf_RL_Lo" :`NewEnumerator1` "/Game/AtmosphereV2/MaterialInstances/Low/Surf_ML_Lo.Surf_ML_Lo" :`NewEnumerator2` "/Game/AtmosphereV2/MaterialInstances/Low/Surf_RML_Lo.Surf_RML_Lo" :!type "MaterialInterface Object Reference"))))

(fn `SelectSurfMaterial_Medium`
  (returns (Material :type "MaterialInterface Object Reference"))
  (bind _scatteringtype (`self.ScatteringType`))
  (return (select `bool` (`self.EnableLighting`) :`false` (select `/Game/AtmosphereV2/System/Blueprints/AtmoBP_ScatteringType` _scatteringtype :`NewEnumerator0` "/Game/AtmosphereV2/MaterialInstances/Medium/Surf_R_Mid.Surf_R_Mid" :`NewEnumerator1` "/Game/AtmosphereV2/MaterialInstances/Medium/Surf_M_Mid.Surf_M_Mid" :`NewEnumerator2` "/Game/AtmosphereV2/MaterialInstances/Medium/Surf_RM_Mid.Surf_RM_Mid" :!type "MaterialInterface Object Reference") :`true` (select `/Game/AtmosphereV2/System/Blueprints/AtmoBP_ScatteringType` _scatteringtype :`NewEnumerator0` "/Game/AtmosphereV2/MaterialInstances/Medium/Surf_RL_Mid.Surf_RL_Mid" :`NewEnumerator1` "/Game/AtmosphereV2/MaterialInstances/Medium/Surf_ML_Mid.Surf_ML_Mid" :`NewEnumerator2` "/Game/AtmosphereV2/MaterialInstances/Medium/Surf_RML_Mid.Surf_RML_Mid" :!type "MaterialInterface Object Reference"))))

(fn `SetMaterialLight`
  (params (MaterialInstance :type "MaterialInstanceDynamic Object Reference"))
  (`|ExecutionSequence`
    (:`then_0`
      (`MaterialInstanceDynamic.SetVectorParameterValue` MaterialInstance "LightDirection" (`KismetMathLibrary.Conv_VectorToLinearColor` (`self.LightDirection`))))
    (:`then_1`
      (`MaterialInstanceDynamic.SetVectorParameterValue` MaterialInstance "LightBrightness" (* (`self.LightColor`) (`self.LightBrightness`))))
    (:`then_2`
      (`MaterialInstanceDynamic.SetVectorParameterValue` MaterialInstance "Skylight" (* (`self.Skylight`) (`self.SkylightIntensity`))))
    (:`then_3`
      (`|ExecutionSequence`
        (:`then_0`
          (`MaterialInstanceDynamic.SetScalarParameterValue` MaterialInstance "SkylightMultiplier" (`self.SkylightMultiplier`)))
        (:`then_1`
          (`MaterialInstanceDynamic.SetScalarParameterValue` MaterialInstance "SkylightConstant" (`self.SkylightConstant`)))
        (:`then_2`
          (`MaterialInstanceDynamic.SetScalarParameterValue` MaterialInstance "SkylightPower" (`self.SkylightPower`)))))))

(fn `SetMaterialRadius`
  (params (`Material Instance` :type "MaterialInstanceDynamic Object Reference") (InnerRadius :type "Float (double-precision)" :default 0.0) (OuterRadius :type "Float (double-precision)" :default 0.0))
  (`|ExecutionSequence`
    (:`then_0`
      (`MaterialInstanceDynamic.SetScalarParameterValue` `Material Instance` "InnerRadius" InnerRadius))
    (:`then_1`
      (`MaterialInstanceDynamic.SetScalarParameterValue` `Material Instance` "OuterRadius" OuterRadius))))

(fn `SetMaterialScattering`
  (params (MaterialInstance :type "MaterialInstanceDynamic Object Reference"))
  (`|ExecutionSequence`
    (:`then_0`
      (`self.SetMaterialScatteringType` MaterialInstance (`self.RayleighScattering`) "Rayleigh"))
    (:`then_1`
      (`self.SetMaterialScatteringType` MaterialInstance (`self.MieScattering`) "Mie"))
    (:`then_2`
      (`MaterialInstanceDynamic.SetScalarParameterValue` MaterialInstance "MieG" (`self.MieG`)))))

(fn `SetMaterialScatteringType`
  (params (MaterialInstance :type "MaterialInstanceDynamic Object Reference") (Parameters :type "/Game/AtmosphereV2/System/Blueprints/AtmoBP_Scattering Structure") (Type :type String))
  (bind (_finalscatter _finalattenuation _finalscaleheight) (`self.CalcScatteringParameters` Parameters))
  (`|ExecutionSequence`
    (:`then_0`
      (`MaterialInstanceDynamic.SetVectorParameterValue` MaterialInstance (`KismetStringLibrary.Conv_StringToName` (`KismetStringLibrary.Concat_StrStr` Type "Scatter")) _finalscatter))
    (:`then_1`
      (`MaterialInstanceDynamic.SetVectorParameterValue` MaterialInstance (`KismetStringLibrary.Conv_StringToName` (`KismetStringLibrary.Concat_StrStr` Type "Attenuation")) _finalattenuation))
    (:`then_2`
      (`MaterialInstanceDynamic.SetScalarParameterValue` MaterialInstance (`KismetStringLibrary.Conv_StringToName` (`KismetStringLibrary.Concat_StrStr` Type "ScaleHeight")) _finalscaleheight))))

(fn `SetOuterRadius`
  (params (OuterRadius :type "Float (double-precision)" :default 0.0))
  (bind _returnvalue (/ OuterRadius (`self.MakeUniformSize` (`.Max` (`StaticMeshComponent.GetLocalBounds`)))))
  (`SceneComponent.SetWorldScale3D` (`KismetMathLibrary.MakeVector` _returnvalue _returnvalue _returnvalue)))

(fn `UserConstructionScript`
  (bind _radius (`self.GetActualPlanetRadius`))
  (bind _outerradius (`self.CalcOuterRadius` _radius))
  (bind (_skymi _surfacemi) (`self.InitMaterials`))
  (`|ExecutionSequence`
    (:`then_0`
      (`self.InitMaterialParameters` _skymi _radius _outerradius))
    (:`then_1`
      (`self.InitMaterialParameters` _surfacemi _radius _outerradius))
    (:`then_2`
      (`self.SetOuterRadius` _outerradius))))